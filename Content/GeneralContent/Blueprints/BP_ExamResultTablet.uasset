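; BP_ExamResultTablet is an actor that displays the player's exam results on a UI_Exam_Report widget component.
; On BeginPlay it caches the widget and runs FreshReport, which reads the results from the Global_Arrays game instance.
; It lists the user's numbered steps, marking those that differ from the correct answer at the same index as wrong order.
; It then adds the correct answers, missing steps and final score.
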(event Custom|FreshReport
  (Utilities|FlowControl|Sequence
    (:then_0
      ;[1 1 1] Show user steps
      (bind _asglobal_arrays (Utilities|Casting|CastToGlobal_Arrays (Game|GetGameInstance)))
      (for (_array_element _array_index) (Variables|/Game/GeneralContent/Blueprints/Global_Arrays.Global_Arrays_C|GetStepDescRecord _asglobal_arrays)
        (if (Utilities|Enum|Equal(Enum) _array_element (Utilities|Array|Get(acopy) (Variables|/Game/GeneralContent/Blueprints/Global_Arrays.Global_Arrays_C|GetCorrectAnswers _asglobal_arrays) _array_index))
          (Default|AddTextinUserStepScrollBox (Variables|Default|GetAs%20UI%20Exam%20Report) (Utilities|String|Append (Utilities|String|Append (Utilities|String|ToString(Integer) (+ _array_index 1)) ". ") _array_element) true)
          (else
            (Default|AddTextinUserStepScrollBox (Variables|Default|GetAs%20UI%20Exam%20Report) (Utilities|String|Append (Utilities|String|Append (Utilities|String|Append (Utilities|String|ToString(Integer) (+ _array_index 1)) ". ") _array_element) "(Wrong Order)") false)))))
    (:then_1
      ;[1 1 1] Show correct answer
      (bind _asglobal_arrays_2 (Utilities|Casting|CastToGlobal_Arrays (Game|GetGameInstance)))
      (for (_array_element_2 _array_index_2) (Variables|/Game/GeneralContent/Blueprints/Global_Arrays.Global_Arrays_C|GetCorrectAnswers _asglobal_arrays_2)
        (Default|AddTextinCorrectAnswerScrollBox (Variables|Default|GetAs%20UI%20Exam%20Report) (Utilities|String|Append (Utilities|String|Append (Utilities|String|ToString(Integer) (+ _array_index_2 1)) ". ") _array_element_2))
        (Development|PrintString (Utilities|String|Append (Utilities|String|Append (Utilities|String|ToString(Integer) (+ _array_index_2 1)) ". ") _array_element_2))))
    (:then_2
      ;[1 1 1] Show missing steps
      (bind _asglobal_arrays_3 (Utilities|Casting|CastToGlobal_Arrays (Game|GetGameInstance)))
      (for _array_element_3 (Variables|/Game/GeneralContent/Blueprints/Global_Arrays.Global_Arrays_C|GetMissingSteps _asglobal_arrays_3)
        (Default|AddTextinMissingStepScrollBox (Variables|Default|GetAs%20UI%20Exam%20Report) _array_element_3)))
    (:then_3
      ;[1 1 1] Show final score
      (bind _asglobal_arrays_4 (Utilities|Casting|CastToGlobal_Arrays (Game|GetGameInstance)))
      (Default|AddScore (Variables|Default|GetAs%20UI%20Exam%20Report) (Variables|/Game/GeneralContent/Blueprints/Global_Arrays.Global_Arrays_C|GetFinalScore _asglobal_arrays_4)))))

(event EventBeginPlay
  (|CallParentFunction)
  (bind _asui_exam_report (Utilities|Casting|CastToUI_Exam_Report (UserInterface|GetUserWidgetObject (Variables|Default|GetExamReport))))
  (Variables|Default|SetAs%20UI%20Exam%20Report _asui_exam_report)
  (CallFunction|FreshReport))

(event Collision|EventActorBeginOverlap
  (params (OtherActor :type Actor%20Object%20Reference))
  (|CallParentFunction OtherActor) ; This node is disabled and will not be called.\nDrag off pins to build functionality.
)

(event EventTick
  (params (DeltaSeconds :type Float%20%28single-precision%29))
  (|CallParentFunction DeltaSeconds) ; This node is disabled and will not be called.\nDrag off pins to build functionality.
)

(fn ConstructionScript
  (|CallParentFunction))